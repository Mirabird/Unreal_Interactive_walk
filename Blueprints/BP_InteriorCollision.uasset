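; Trigger volume that switches the world between interior and exterior states as something enters or leaves its SM_IntCollision mesh.
; Entering streams in interior furniture, lighting and plants, unloads exterior lighting, fake light and foliage levels, re-aims the SunSky directional light and hides instanced foliage.
; Leaving reverses this.
; Both transitions show the first-person character's preloader widget, hidden again after a short fixed delay rather than on load completion.
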(event `self.SM_IntCollision.OnComponentBeginOverlap`
  (params (OverlappedComponent :type "PrimitiveComponent Object Reference") (OtherActor :type "Actor Object Reference") (OtherComp :type "PrimitiveComponent Object Reference") (OtherBodyIndex :type Integer) (bFromSweep :type Boolean) (SweepResult :type "HitResult Structure (by ref)"))
  ;[1 1 1] PreloaderVisible
  (bind _asbp_first_person_character (cast `/Game/FirstPerson/Blueprints/BP_FirstPersonCharacter` (`GameplayStatics.GetPlayerPawn` 0)))
  (bind _preloaderref (`/Game/FirstPerson/Blueprints/BP_FirstPersonCharacter.PreloaderRef` _asbp_first_person_character))
  (`Widget.SetVisibility` _preloaderref "Visible")
  ;[1 1 1] LoadUnloadLevels
  (`GameplayStatics.LoadStreamLevelBySoftObjectPtr` "/Game/Levels/InteriorFurniture.InteriorFurniture" true)
  (`GameplayStatics.LoadStreamLevelBySoftObjectPtr` "/Game/Levels/InteriorLight.InteriorLight" true)
  (`GameplayStatics.UnloadStreamLevelBySoftObjectPtr` "/Game/Levels/ExteriorLight.ExteriorLight")
  (`GameplayStatics.UnloadStreamLevelBySoftObjectPtr` "/Game/Levels/FakeLight.FakeLight")
  (`GameplayStatics.UnloadStreamLevelBySoftObjectPtr` "/Game/Levels/Foliage.Foliage")
  (bind _returnvalue (`GameplayStatics.GetActorOfClass` "/SunPosition/SunSky.SunSky_C"))
  (`SceneComponent.K2_SetWorldRotation` (`/SunPosition/SunSky.DirectionalLight` _returnvalue) (struct :`Pitch` -32.81 :`Yaw` -169.13 :`Roll` 180.0) false false)
  (bind _returnvalue_2 (`GameplayStatics.GetActorOfClass` "/Script/Foliage.InstancedFoliageActor"))
  (`self.SetActorHiddenInGame` _returnvalue_2 true)
  (`GameplayStatics.LoadStreamLevelBySoftObjectPtr` "/Game/Levels/Plants.Plants" true)
  ;[1 1 1] PreloaderHidden
  (`KismetSystemLibrary.Delay` 0.2)
  (`Widget.SetVisibility` _preloaderref "Hidden"))

(event `self.SM_IntCollision.OnComponentEndOverlap`
  (params (OverlappedComponent :type "PrimitiveComponent Object Reference") (OtherActor :type "Actor Object Reference") (OtherComp :type "PrimitiveComponent Object Reference") (OtherBodyIndex :type Integer))
  (bind _asbp_first_person_character (cast `/Game/FirstPerson/Blueprints/BP_FirstPersonCharacter` (`GameplayStatics.GetPlayerPawn` 0)))
  (bind _preloaderref (`/Game/FirstPerson/Blueprints/BP_FirstPersonCharacter.PreloaderRef` _asbp_first_person_character))
  (`Widget.SetVisibility` _preloaderref "Visible")
  (`GameplayStatics.LoadStreamLevelBySoftObjectPtr` "/Game/Levels/ExteriorLight.ExteriorLight" true)
  (`GameplayStatics.LoadStreamLevelBySoftObjectPtr` "/Game/Levels/FakeLight.FakeLight" true)
  (`GameplayStatics.LoadStreamLevelBySoftObjectPtr` "/Game/Levels/Foliage.Foliage" true)
  (`GameplayStatics.UnloadStreamLevelBySoftObjectPtr` "/Game/Levels/InteriorFurniture.InteriorFurniture")
  (`GameplayStatics.UnloadStreamLevelBySoftObjectPtr` "/Game/Levels/InteriorLight.InteriorLight")
  (bind _returnvalue (`GameplayStatics.GetActorOfClass` "/SunPosition/SunSky.SunSky_C"))
  (`SceneComponent.K2_SetWorldRotation` (`/SunPosition/SunSky.DirectionalLight` _returnvalue) (struct :`Pitch` -7.51 :`Yaw` -133.7 :`Roll` -180.0) false false)
  (bind _returnvalue_2 (`GameplayStatics.GetActorOfClass` "/Script/Foliage.InstancedFoliageActor"))
  (`self.SetActorHiddenInGame` _returnvalue_2 false)
  (`GameplayStatics.UnloadStreamLevelBySoftObjectPtr` "/Game/Levels/Plants.Plants")
  (`KismetSystemLibrary.Delay` 0.2)
  (`Widget.SetVisibility` _preloaderref "Hidden"))

(fn `UserConstructionScript`)